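; BP_SnakeRanged is a ranged snake enemy that fires a poison attack in time with its sprite animation.
; Each Tick, it watches the SnakeAttack1 flipbook and, from frame 84 onward, spawns BP_PoisonAttack at the actor's rotation, offset along the X component of its forward vector.
; The PoisonCreated flag limits this to one spawn per playback, resetting while that flipbook is before the firing frame.
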(event EventBeginPlay
  (|CallParentFunction) ; This node is disabled and will not be called.\nDrag off pins to build functionality.
)

(event Collision|EventActorBeginOverlap
  (params (OtherActor :type Actor%20Object%20Reference))
  (|CallParentFunction OtherActor) ; This node is disabled and will not be called.\nDrag off pins to build functionality.
)

(event EventTick
  (params (DeltaSeconds :type Float%20%28single-precision%29))
  (bind _returnvalue (Transformation|GetActorRotation))
  (bind _sprite (Variables|Default|GetSprite))
  (if (== (Class|PaperFlipbookComponent|GetFlipbook _sprite) "/Game/GirafficPark/Assets/Snake_Attack1/SnakeAttack1.SnakeAttack1")
    (if (>= (Class|PaperFlipbookComponent|GetPlaybackPositioninFrames _sprite) 84)
      (if (not (Variables|Default|GetPoisonCreated))
        (Game|SpawnActorfromClass "/Game/GirafficPark/BP/Weapons/BP_PoisonAttack.BP_PoisonAttack_C" (Math|Transform|MakeTransform (+ (Transformation|GetActorLocation) (* (Math|Vector|GetForwardVector _returnvalue) "15.000000,0.000000,0.000000")) _returnvalue "1.000000,1.000000,1.000000") "Undefined" "MultiplyWithRoot" 0 0)
        (Variables|Default|SetPoisonCreated true))
      (else
        (Variables|Default|SetPoisonCreated false)))))

(fn ConstructionScript
  (|CallParentFunction))