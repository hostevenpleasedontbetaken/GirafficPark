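; Pangolin enemy with a flipbook sprite that rolls into a ball when the player comes near, then moves along a set direction.
; The Proximity overlap plays the roll-up flipbook once, then switches to the rolling one.
; Tick waits one second before starting continuous unswept movement, spinning the sprite by a fixed step each frame.
; A separate Damage overlap calls PlayerHit when it touches the player.
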(event OnComponentBeginOverlap(Damage)
  (params (OverlappedComponent :type Primitive%20Component%20Object%20Reference) (OtherActor :type Actor%20Object%20Reference) (OtherComp :type Primitive%20Component%20Object%20Reference) (OtherBodyIndex :type Integer) (bFromSweep :type Boolean) (SweepResult :type Hit%20Result%20Structure%20%28by%20ref%29))
  (if (Collision|IsOverlappingActor OverlappedComponent (Game|GetPlayerCharacter 0) :!class /Script/Engine.PrimitiveComponent)
    (CallFunction|PlayerHit true)))

(event OnComponentBeginOverlap(Proximity)
  (params (OverlappedComponent :type Primitive%20Component%20Object%20Reference) (OtherActor :type Actor%20Object%20Reference) (OtherComp :type Primitive%20Component%20Object%20Reference) (OtherBodyIndex :type Integer) (bFromSweep :type Boolean) (SweepResult :type Hit%20Result%20Structure%20%28by%20ref%29))
  (if (Collision|IsOverlappingActor OverlappedComponent (Game|GetPlayerCharacter 0) :!class /Script/Engine.PrimitiveComponent)
    (if (not (Variables|Default|GetRolledUp))
      (Variables|Default|SetOverlapped true)
      (Sprite|SetFlipbook (Variables|Default|GetSprite) "/Game/GirafficPark/Assets/Pangolin_RollUp/RollUp.RollUp")
      (Variables|Default|SetRolledUp true)
      (Utilities|FlowControl|Delay (Class|PaperFlipbookComponent|GetFlipbookLength (Variables|Default|GetSprite)))
      (Sprite|SetFlipbook (Variables|Default|GetSprite) "/Game/GirafficPark/Assets/Pangolin_Attack/Pangolin_Roll.Pangolin_Roll"))))

(event EventBeginPlay
  (|CallParentFunction) ; This node is disabled and will not be called.\nDrag off pins to build functionality.
)

(event EventTick
  (params (DeltaSeconds :type Float%20%28single-precision%29))
  (if (Variables|Default|GetOverlapped)
    (if (Variables|Default|GetDelay)
      (Transformation|AddActorWorldOffset (* DeltaSeconds (* (Variables|Default|GetMoveDirection) (Variables|Default|GetMoveSpeed))))
      (Transformation|AddLocalRotation (Variables|Default|GetSprite) "10.000000,0.000000,0.000000" false false)
      (else
        (Utilities|FlowControl|Delay 1.0)
        (Transformation|AddActorWorldOffset (* DeltaSeconds (* (Variables|Default|GetMoveDirection) (Variables|Default|GetMoveSpeed))))
        (Variables|Default|SetDelay true)))))

(fn ConstructionScript
  (|CallParentFunction))