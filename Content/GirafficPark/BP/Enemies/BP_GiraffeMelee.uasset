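; Paper2D melee giraffe enemy that walks along its forward vector while its Overlapped flag is set and kicks the player.
; Player proximity switches to the kick flipbook and enables the attack box until a timer restores walking.
; Tick calls PlayerHit for player characters in that box only during a mid-kick frame window.
; Hitting dirt, sand platforms or moveable boxes turns it around, with a short delay preventing repeated flips.
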(event OnComponentBeginOverlap(Damage)
  (params (OverlappedComponent :type Primitive%20Component%20Object%20Reference) (OtherActor :type Actor%20Object%20Reference) (OtherComp :type Primitive%20Component%20Object%20Reference) (OtherBodyIndex :type Integer) (bFromSweep :type Boolean) (SweepResult :type Hit%20Result%20Structure%20%28by%20ref%29))
  (bind _returnvalue (Transformation|GetActorRotation))
  (Utilities|Casting|CastToSolidDirt OtherActor
    (:then
      _)
    (:CastFailed
      (Utilities|Casting|CastToSandPlatform OtherActor
        (:then
          _)
        (:CastFailed
          (Utilities|Casting|CastToMoveableBox OtherActor)))))
  (if (not (Variables|Default|GetRotated))
    (Variables|Default|SetRotated true)
    (Transformation|SetActorRotation (Math|Rotator|MakeRotator (.roll _returnvalue) (.pitch _returnvalue) (+ (.yaw _returnvalue) 1.8e+02)))
    (Utilities|FlowControl|Delay 0.5)
    (Variables|Default|SetRotated false)))

(event OnComponentBeginOverlap(AttackProx)
  (params (OverlappedComponent :type Primitive%20Component%20Object%20Reference) (OtherActor :type Actor%20Object%20Reference) (OtherComp :type Primitive%20Component%20Object%20Reference) (OtherBodyIndex :type Integer) (bFromSweep :type Boolean) (SweepResult :type Hit%20Result%20Structure%20%28by%20ref%29))
  (if (Collision|IsOverlappingActor OverlappedComponent (Game|GetPlayerCharacter 0) :!class /Script/Engine.PrimitiveComponent)
    (if (not (Variables|Default|GetAttack))
      (Variables|Default|SetAttack true)
      (CallFunction|AttackonAnimation))))

(event Custom|AttackOnAnimation
  (Sprite|SetFlipbook (Variables|Default|GetSprite) "/Game/GirafficPark/Assets/GiraffeAttack2/GiraffeKick.GiraffeKick")
  (Collision|SetCollisionEnabled (Variables|Components|GetAttackBox) "QueryAndPhysics")
  (Utilities|Time|SetTimerbyEvent (delegate Custom|Reset%20Animation) (Class|PaperFlipbookComponent|GetFlipbookLength (Variables|Default|GetSprite))))

(event Custom|Reset%20Animation
  (Sprite|SetFlipbook (Variables|Default|GetSprite) "/Game/GirafficPark/Assets/GiraffeWalk/GiraffeWalk.GiraffeWalk")
  (Collision|SetCollisionEnabled (Variables|Components|GetAttackBox) "NoCollision")
  (Variables|Default|SetAttack false))

(event EventBeginPlay
  (|CallParentFunction) ; This node is disabled and will not be called.\nDrag off pins to build functionality.
)

(event Collision|EventActorBeginOverlap
  (params (OtherActor :type Actor%20Object%20Reference))
  (|CallParentFunction OtherActor) ; This node is disabled and will not be called.\nDrag off pins to build functionality.
)

(event EventTick
  (params (DeltaSeconds :type Float%20%28single-precision%29))
  (bind _returnvalue (Transformation|GetActorForwardVector))
  (bind _sprite (Variables|Default|GetSprite))
  (bind _returnvalue_2 (Class|PaperFlipbookComponent|GetPlaybackPositioninFrames _sprite))
  (if (Variables|Default|GetOverlapped)
    (if (Variables|Default|GetAttack)
      (if (== (Class|PaperFlipbookComponent|GetFlipbook _sprite) "/Game/GirafficPark/Assets/GiraffeAttack2/GiraffeKick.GiraffeKick")
        (if (and (> _returnvalue_2 22) (< _returnvalue_2 32))
          (for _array_element (Collision|GetOverlappingActors (Variables|Components|GetAttackBox) "/Game/GirafficPark/BP/Player/BP_PaperCharacter.BP_PaperCharacter_C" :!class /Script/Engine.PrimitiveComponent)
            (CallFunction|PlayerHit true))))
      (else
        (Transformation|AddActorWorldOffset (* DeltaSeconds (* (Math|Vector|MakeVector 0.0 (.y _returnvalue) (.z _returnvalue)) (* (Variables|Default|GetMoveSpeed) (Variables|Default|GetDirectionRotator)))))))))

(fn ConstructionScript
  (|CallParentFunction))