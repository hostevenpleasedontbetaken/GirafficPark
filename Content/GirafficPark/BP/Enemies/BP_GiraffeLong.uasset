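; BP_GiraffeLong is a flipbook-animated giraffe enemy that advances and performs a timed attack when the player comes within range.
; Tick moves it along MoveDirection without sweeping while Overlapped is true and it is not attacking; this graph never sets Overlapped.
; An AttackProx overlap with the player plays the attack flipbook and enables AttackBox collision.
; A timer matching the flipbook's length then restores the Frogidle flipbook, disables the hitbox and clears Attack.
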(event OnComponentBeginOverlap(AttackProx)
  (params (OverlappedComponent :type Primitive%20Component%20Object%20Reference) (OtherActor :type Actor%20Object%20Reference) (OtherComp :type Primitive%20Component%20Object%20Reference) (OtherBodyIndex :type Integer) (bFromSweep :type Boolean) (SweepResult :type Hit%20Result%20Structure%20%28by%20ref%29))
  (if (Collision|IsOverlappingActor OverlappedComponent (Game|GetPlayerCharacter 0) :!class /Script/Engine.PrimitiveComponent)
    (Variables|Default|SetAttack true)
    (CallFunction|AttackonAnimation)))

(event Custom|AttackOnAnimation
  (Sprite|SetFlipbook (Variables|Default|GetSprite) "/Game/GirafficPark/Assets/Giraffe_Attack1/Giraffe_Attack1.Giraffe_Attack1")
  (Collision|SetCollisionEnabled (Variables|Default|GetAttackBox) "QueryAndPhysics")
  (Utilities|Time|SetTimerbyEvent (delegate Custom|Reset%20Animation) (Class|PaperFlipbookComponent|GetFlipbookLength (Variables|Default|GetSprite))))

(event Custom|Reset%20Animation
  (Sprite|SetFlipbook (Variables|Default|GetSprite) "/Game/GirafficPark/TestAssets/PNG/sprites/frog/idle/frog-idle.frog-idle")
  (Collision|SetCollisionEnabled (Variables|Default|GetAttackBox) "NoCollision")
  (Variables|Default|SetAttack false))

(event EventBeginPlay
  (|CallParentFunction) ; This node is disabled and will not be called.\nDrag off pins to build functionality.
)

(event Collision|EventActorBeginOverlap
  (params (OtherActor :type Actor%20Object%20Reference))
  (|CallParentFunction OtherActor) ; This node is disabled and will not be called.\nDrag off pins to build functionality.
)

(event EventTick
  (params (DeltaSeconds :type Float%20%28single-precision%29))
  (if (Variables|Default|GetOverlapped)
    (if (not (Variables|Default|GetAttack))
      (Transformation|AddActorWorldOffset (* DeltaSeconds (* (Variables|Default|GetMoveDirection) (Variables|Default|GetMoveSpeed)))))))

(fn ConstructionScript
  (|CallParentFunction))