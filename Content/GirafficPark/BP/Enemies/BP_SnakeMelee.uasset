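; BP_SnakeMelee is a 2D Paper2D snake enemy that performs a timed melee attack against the player.
; A looping timer set on BeginPlay plays the attack flipbook every two seconds, then restores idle once it finishes.
; Tick watches a narrow frame window of that flipbook, enabling query collision on the Attack component and calling PlayerHit for overlapping player characters.
; The collision is never disabled again here.
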(event Custom|SnakeAttack
  (bind _sprite (Variables|Default|GetSprite))
  (Sprite|SetFlipbook _sprite "/Game/GirafficPark/Assets/Snake_Attack1/SnakeAttack1.SnakeAttack1")
  (Utilities|FlowControl|Delay (Class|PaperFlipbookComponent|GetFlipbookLength _sprite))
  (Sprite|SetFlipbook (Variables|Default|GetSprite) "/Game/GirafficPark/Assets/Snake_Idle/SNake_Idle.SNake_Idle"))

(event EventBeginPlay
  (Utilities|Time|SetTimerbyEvent (delegate Custom|SnakeAttack) 2.0 true)
  (|CallParentFunction))

(event Collision|EventActorBeginOverlap
  (params (OtherActor :type Actor%20Object%20Reference))
  (|CallParentFunction OtherActor) ; This node is disabled and will not be called.\nDrag off pins to build functionality.
)

(event EventTick
  (params (DeltaSeconds :type Float%20%28single-precision%29))
  (bind _sprite (Variables|Default|GetSprite))
  (bind _returnvalue (Class|PaperFlipbookComponent|GetPlaybackPositioninFrames _sprite))
  (if (== (Class|PaperFlipbookComponent|GetFlipbook _sprite) "/Game/GirafficPark/Assets/Snake_Attack1/SnakeAttack1.SnakeAttack1")
    (if (and (> _returnvalue 88) (< _returnvalue 96))
      (Collision|SetCollisionEnabled (Variables|Default|GetAttack) "QueryOnly")
      (CallFunction|HitCHeck))))

(fn ConstructionScript
  (|CallParentFunction))

(fn HitCHeck
  (for _array_element (Collision|GetOverlappingActors (Variables|Default|GetAttack) "/Game/GirafficPark/BP/Player/BP_PaperCharacter.BP_PaperCharacter_C" :!class /Script/Engine.PrimitiveComponent)
    (CallFunction|PlayerHit true)))