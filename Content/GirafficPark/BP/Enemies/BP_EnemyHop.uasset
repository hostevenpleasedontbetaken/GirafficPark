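; BP_EnemyHop is a hopping enemy that moves along its move direction and shows rabbit jump or landing animations.
; While its Overlapped flag is true, Tick offsets the actor without sweep, derives vertical speed from frame-to-frame height change and compares it to thresholds to switch the sprite's flipbook.
; The file never sets that flag or launches a hop.
; An unconnected frog animation branch based on CharacterMovement falling state never runs.
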(event EventBeginPlay
  (|CallParentFunction) ; This node is disabled and will not be called.\nDrag off pins to build functionality.
)

(event Collision|EventActorBeginOverlap
  (params (OtherActor :type Actor%20Object%20Reference))
  (|CallParentFunction OtherActor) ; This node is disabled and will not be called.\nDrag off pins to build functionality.
)

(event EventTick
  (params (DeltaSeconds :type Float%20%28single-precision%29))
  (if (Variables|Default|GetOverlapped)
    (Transformation|AddActorWorldOffset (* DeltaSeconds (* (Variables|Default|GetMoveDirection) (Variables|Default|GetMoveSpeed))))
    (bind _output_get (Variables|Default|SetCurrentZ (.z (Transformation|GetActorLocation))))
    (bind _output_get_2 (Variables|Default|SetZVel (/ (- _output_get (Variables|Default|GetPreviousZ)) DeltaSeconds)))
    (Variables|Default|SetPreviousZ (Variables|Default|GetCurrentZ))
    (if (> _output_get_2 (Variables|Default|GetJumpThreshold))
      (Sprite|SetFlipbook (Variables|Default|GetSprite) "/Game/GirafficPark/Assets/Rabbit/RabbitJump.RabbitJump")
      (elif (< _output_get_2 (Variables|Default|GetFallThreshold))
        (Sprite|SetFlipbook (Variables|Default|GetSprite) "/Game/GirafficPark/Assets/Rabbit/RabbitLand.RabbitLand")))))

(fn ConstructionScript
  (|CallParentFunction))