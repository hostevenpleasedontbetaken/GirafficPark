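; Zookeeper enemy, apparently a boss, that walks while Overlapped is set and turns around on bumping dirt, sand platforms or boxes.
; A looping ChooseAttack timer chain picks a net swing in melee range, otherwise randomly a poison dart burst or SealBazooka, which only plays a throw animation.
; Tick checks flipbook frame windows during the net swing to test short, medium and long hit boxes against the player.
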(event OnComponentBeginOverlap(Damage)
  (params (OverlappedComponent :type Primitive%20Component%20Object%20Reference) (OtherActor :type Actor%20Object%20Reference) (OtherComp :type Primitive%20Component%20Object%20Reference) (OtherBodyIndex :type Integer) (bFromSweep :type Boolean) (SweepResult :type Hit%20Result%20Structure%20%28by%20ref%29))
  (bind _returnvalue (Transformation|GetActorRotation))
  ;[1 1 1 1 100] ROTATE On Bump
  (Utilities|Casting|CastToSolidDirt OtherActor
    (:then
      _)
    (:CastFailed
      (Utilities|Casting|CastToSandPlatform OtherActor
        (:then
          _)
        (:CastFailed
          (Utilities|Casting|CastToMoveableBox OtherActor)))))
  (if (not (Variables|Default|GetRotated))
    (Variables|Default|SetRotated true)
    (Transformation|SetActorRotation (Math|Rotator|MakeRotator (.roll _returnvalue) (.pitch _returnvalue) (+ (.yaw _returnvalue) 1.8e+02)))
    (Utilities|FlowControl|Delay 0.5)
    (Variables|Default|SetRotated false)))

(event OnComponentEndOverlap(AttackProx)
  (params (OverlappedComponent :type Primitive%20Component%20Object%20Reference) (OtherActor :type Actor%20Object%20Reference) (OtherComp :type Primitive%20Component%20Object%20Reference) (OtherBodyIndex :type Integer))
  ;[1 1 1] MeleeRangeCHeck
  (if (Collision|IsOverlappingActor OverlappedComponent (Game|GetPlayerCharacter 0) :!class /Script/Engine.PrimitiveComponent)
    (Variables|Default|SetMeleeRange false)))

(event OnComponentBeginOverlap(AttackProx)
  (params (OverlappedComponent :type Primitive%20Component%20Object%20Reference) (OtherActor :type Actor%20Object%20Reference) (OtherComp :type Primitive%20Component%20Object%20Reference) (OtherBodyIndex :type Integer) (bFromSweep :type Boolean) (SweepResult :type Hit%20Result%20Structure%20%28by%20ref%29))
  ;[1 1 1] MeleeRangeCHeck
  (if (Collision|IsOverlappingActor OverlappedComponent (Game|GetPlayerCharacter 0) :!class /Script/Engine.PrimitiveComponent)
    (Variables|Default|SetMeleeRange true)))

(event Custom|AttackOnAnimation
  (bind _returnvalue (Transformation|GetActorLocation))
  ;[1 1 1 1 100] AttackAnimation
  (bind _returnvalue_2 (Actor|GetActorOfClass "/Game/GirafficPark/BP/Player/BP_PaperCharacter.BP_PaperCharacter_C"))
  (if (< (.x (Transformation|GetActorLocation _returnvalue_2)) (.x _returnvalue))
    (Transformation|SetActorRotation (Math|Rotator|MakeRotator (.x _returnvalue) (.y _returnvalue) 0.0))
    (else
      (Transformation|SetActorRotation (Math|Rotator|MakeRotator (.x _returnvalue) (.y _returnvalue) 1.8e+02))))
  (Sprite|SetFlipbook (Variables|Default|GetSprite) "/Game/GirafficPark/Assets/Zookeeper/Net/KeeperNet.KeeperNet")
  (Utilities|Time|SetTimerbyEvent (delegate Custom|Reset%20Animation) (Class|PaperFlipbookComponent|GetFlipbookLength (Variables|Default|GetSprite))))

(event Custom|Reset%20Animation
  ;[1 1 1 1 100] AttackAnimation
  (Sprite|SetFlipbook (Variables|Default|GetSprite) "/Game/GirafficPark/Assets/Zookeeper/Idle/keeperidle.keeperidle")
  (Collision|SetCollisionEnabled (Variables|Components|GetMedAttackBox) "NoCollision")
  (Variables|Default|SetAttack false)
  (Utilities|Time|SetTimerbyFunctionName 0 "ChooseAttack" 3.0))

(event Custom|UpdateZooAnimation
  (if (not (Variables|Default|GetAttack))
    (Sprite|SetFlipbook (Variables|Default|GetSprite) "/Game/GirafficPark/Assets/Zookeeper/Walk/KeeperWalk.KeeperWalk")))

(event Custom|EachDartRount
  (bind _result (Math|Integer|IncrementInt (Variables|Default|GetDartRounds))
    (:%20%20
      (Development|PrintString (Utilities|String|ToString(Integer) _result))
      (if (not (< (Variables|Default|GetDartRounds) 4))
        (Utilities|Time|ClearandInvalidateTimerbyHandle (Variables|Default|GetDartRoundHandle))
        (Variables|Default|SetDartRounds 0)
        (Variables|Default|SetBurstFireCount 0)))))

(event Custom|SealBazooka
  (bind _sprite (Variables|Default|GetSprite))
  ;[1 1 1 1 100] Seal Bazooka
  (Sprite|SetFlipbook _sprite "/Game/GirafficPark/Assets/Zookeeper/Throw/KeeperThrow.KeeperThrow")
  (Utilities|FlowControl|Delay (Class|PaperFlipbookComponent|GetFlipbookLength _sprite))
  (Sprite|SetFlipbook _sprite "/Game/GirafficPark/Assets/Zookeeper/Idle/keeperidle.keeperidle")
  (Variables|Default|SetAttack false)
  (Utilities|Time|SetTimerbyFunctionName 0 "ChooseAttack" 3.0))

(event EventBeginPlay
  ;[1 1 1 1 100] BeginPlay / Select Attack
  (Utilities|Time|SetTimerbyFunctionName 0 "ChooseAttack" 3.0))

(event Collision|EventActorBeginOverlap
  (params (OtherActor :type Actor%20Object%20Reference))
  (|CallParentFunction OtherActor))

(event EventTick
  (params (DeltaSeconds :type Float%20%28single-precision%29))
  (bind _sprite (Variables|Default|GetSprite))
  (bind _sprite_2 (Variables|Default|GetSprite))
  (bind _sprite_3 (Variables|Default|GetSprite))
  (bind _returnvalue (Class|PaperFlipbookComponent|GetPlaybackPositioninFrames _sprite_2))
  (bind _returnvalue_2 (Class|PaperFlipbookComponent|GetPlaybackPositioninFrames _sprite_3))
  (bind _returnvalue_3 (Class|PaperFlipbookComponent|GetPlaybackPositioninFrames _sprite))
  ;[1 1 1 1 100] EVENT TICK
  (if (Variables|Default|GetOverlapped)
    (if (Variables|Default|GetAttack)
      (if (== (Class|PaperFlipbookComponent|GetFlipbook (Variables|Default|GetSprite)) "/Game/GirafficPark/Assets/Zookeeper/Net/KeeperNet.KeeperNet")
        (if (and (> _returnvalue 58) (< _returnvalue 67))
          (CallFunction|MeleeHitCheck)
          (elif (and (> _returnvalue_2 97) (< _returnvalue_2 112))
            (CallFunction|MeleeHitCheck 1)
            (elif (and (> _returnvalue_3 136) (< _returnvalue_3 168))
              (CallFunction|MeleeHitCheck 2)))))
      (else
        (Transformation|AddActorWorldOffset (* DeltaSeconds (* (Transformation|GetActorForwardVector) (* (Variables|Default|GetMoveSpeed) (Variables|Default|GetDirectionRotator)))))
        (CallFunction|UpdateZooAnimation)))))

(fn ConstructionScript
  (|CallParentFunction))

(fn FireBlowDartRound
  (Sprite|SetFlipbook (Variables|Default|GetSprite) "/Game/GirafficPark/Assets/Zookeeper/Throw/KeeperThrow.KeeperThrow")
  (bind _returnvalue (Actor|GetActorOfClass "/Game/GirafficPark/BP/Player/BP_PaperCharacter.BP_PaperCharacter_C"))
  (Variables|Default|SetDartLocation (+ (Transformation|GetActorLocation) (* (Math|Vector|Normalize (- (Transformation|GetActorLocation _returnvalue) (Transformation|GetActorLocation))) "15.000000,0.000000,0.000000")))
  (Variables|Default|SetDartRotation (Math|Rotator|MakeRotfromX (Math|Vector|Normalize (- (Transformation|GetActorLocation _returnvalue) (Transformation|GetActorLocation)))))
  (bind _returnvalue_2 (Utilities|Time|SetTimerbyFunctionName 0 "ShootDart" 0.2 true))
  (Variables|Default|SetBurstFireHandle _returnvalue_2)
  (Utilities|Time|SetTimerbyFunctionName 0 "ChooseAttack" 3.0))

(fn ShootDart
  (Math|Integer|IncrementInt (Variables|Default|GetBurstFireCount)
    (:%20%20
      (if (> (Variables|Default|GetBurstFireCount) 4)
        (Variables|Default|SetBurstFireCount 0)
        (Utilities|Time|ClearandInvalidateTimerbyHandle (Variables|Default|GetBurstFireHandle))
        (else
          (Game|SpawnActorfromClass "/Game/GirafficPark/BP/Weapons/BP_PoisonAttack.BP_PoisonAttack_C" (Math|Transform|MakeTransform (Variables|Default|GetDartLocation) (Variables|Default|GetDartRotation) "1.000000,1.000000,1.000000") "Undefined" "MultiplyWithRoot" 0 0))))))

(fn MeleeHitCheck
  (params (AttackBox :type Integer))
  (switch int AttackBox
    (:0
      (for _array_element (Collision|GetOverlappingActors (Variables|Default|GetShortAttackBox) "/Game/GirafficPark/BP/Player/BP_PaperCharacter.BP_PaperCharacter_C" :!class /Script/Engine.PrimitiveComponent)
        (CallFunction|PlayerHit true)))
    (:1
      (for _array_element_2 (Collision|GetOverlappingActors (Variables|Components|GetMedAttackBox) "/Game/GirafficPark/BP/Player/BP_PaperCharacter.BP_PaperCharacter_C" :!class /Script/Engine.PrimitiveComponent)
        (CallFunction|PlayerHit true)))
    (:2
      (for _array_element_3 (Collision|GetOverlappingActors (Variables|Default|GetLongAttackBox) "/Game/GirafficPark/BP/Player/BP_PaperCharacter.BP_PaperCharacter_C" :!class /Script/Engine.PrimitiveComponent)
        (CallFunction|PlayerHit true)))))

(fn ChooseAttack
  (Variables|Default|SetAttack true)
  (if (Variables|Default|GetMeleeRange)
    (CallFunction|AttackonAnimation)
    (else
      (switch int (Math|Random|RandomIntegerinRange 0 1)
        (:0
          (CallFunction|FireBlowDartRound))
        (:1
          (CallFunction|SealBazooka))))))