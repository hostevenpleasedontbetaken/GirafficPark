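; Player controller for Giraffic Park that sets up mouse input and opens menu screens.
; On BeginPlay it shows the cursor and uses Game and UI input mode.
; The Equip action and a test gift action each switch to UI-only input, add a dimming layer widget, then open and store the equip or gift shop widget.
; It contains no logic for closing those menus or restoring input.
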(event EventBeginPlay
  (Variables|Default|SetbShowMouseCursor true)
  (Input|SetInputModeGameandUI (Game|GetPlayerController 0) 0 "DoNotLock" true false))

(event Input|ActionEvents|InputActionEquip
  (params (Key :type Key%20Structure :default "None"))
  (:Pressed
    (Input|SetInputModeUIOnly self 0 "DoNotLock" false)
    (bind _returnvalue (UserInterface|CreateWidget "/Game/GirafficPark/BP/Widgets/w_DimLayer.w_DimLayer_C"))
    (UserInterface|Viewport|AddtoViewport _returnvalue 0)
    (bind _returnvalue_2 (UserInterface|CreateWidget "/Game/GirafficPark/BP/Widgets/LevelSelectWidgets/W_EquipUI.W_EquipUI_C"))
    (UserInterface|Viewport|AddtoViewport _returnvalue_2 0)
    (Variables|Default|SetEquipUI _returnvalue_2)))

(event Input|ActionEvents|InputActionTESTFORGIFT
  (params (Key :type Key%20Structure :default "None"))
  (:Pressed
    (Input|SetInputModeUIOnly self 0 "DoNotLock" false)
    (bind _returnvalue (UserInterface|CreateWidget "/Game/GirafficPark/BP/Widgets/w_DimLayer.w_DimLayer_C"))
    (UserInterface|Viewport|AddtoViewport _returnvalue 0)
    (bind _returnvalue_2 (UserInterface|CreateWidget "/Game/GirafficPark/BP/Widgets/LevelSelectWidgets/W_GiftShop.W_GiftShop_C"))
    (UserInterface|Viewport|AddtoViewport _returnvalue_2 0)
    (Variables|Default|SetGiftUI _returnvalue_2)))

(fn ConstructionScript)