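; BP_FireBall is a short-lived secondary weapon fireball that damages enemies inside its sphere.
; On BeginPlay it reads its damage from the secondary weapon data in BP_GameInstance, then destroys itself after a brief delay.
; Tick applies that full damage to every overlapping CBP_EnemyBase actor each frame, so total damage depends on frame rate.
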(event EventBeginPlay
  (bind _asbp_game_instance (Utilities|Casting|CastToBP_GameInstance (Game|GetGameInstance)))
  (Variables|Default|SetDamage (.Damage (Utilities|Struct|BreakS_WeaponData (Variables|/Game/GirafficPark/BP/BP_GameInstance.BP_GameInstance_C|GetSecondary%20Weapon _asbp_game_instance))))
  (Utilities|FlowControl|Delay 2.0)
  (Actor|DestroyActor))

(event Collision|EventActorBeginOverlap
  (params (OtherActor :type Actor%20Object%20Reference)))

(event EventTick
  (params (DeltaSeconds :type Float%20%28single-precision%29))
  (for _array_element (Collision|GetOverlappingActors (Variables|Default|GetSphere) "/Game/GirafficPark/BP/Enemies/CBP_EnemyBase.CBP_EnemyBase_C" :!class /Script/Engine.PrimitiveComponent)
    (Game|Damage|ApplyDamage _array_element (Variables|Default|GetDamage) 0 0)))

(fn ConstructionScript)