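; Paper enemy that starts moving once the player enters its Proximity trigger, then keeps going along MoveDirection at MoveSpeed on Tick without sweep.
; Its Damage trigger costs BP_PaperCharacter a life, refreshes the MainGamePlayUI text and launches the player away horizontally and upward.
; Each hit briefly disables input and sets the character's SafePeriod flag, blocking further damage until the delays finish.
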(event OnComponentBeginOverlap(Proximity)
  (params (OverlappedComponent :type Primitive%20Component%20Object%20Reference) (OtherActor :type Actor%20Object%20Reference) (OtherComp :type Primitive%20Component%20Object%20Reference) (OtherBodyIndex :type Integer) (bFromSweep :type Boolean) (SweepResult :type Hit%20Result%20Structure%20%28by%20ref%29))
  (if (Collision|IsOverlappingActor OverlappedComponent (Game|GetPlayerCharacter 0) :!class /Script/Engine.PrimitiveComponent)
    (Variables|Default|SetOverlapped true)
    (Development|PrintString "Hello")))

(event OnComponentBeginOverlap(Damage)
  (params (OverlappedComponent :type Primitive%20Component%20Object%20Reference) (OtherActor :type Actor%20Object%20Reference) (OtherComp :type Primitive%20Component%20Object%20Reference) (OtherBodyIndex :type Integer) (bFromSweep :type Boolean) (SweepResult :type Hit%20Result%20Structure%20%28by%20ref%29))
  (bind _returnvalue (Game|GetPlayerCharacter 0))
  (bind _returnvalue_2 (Actor|GetActorOfClass "/Game/GirafficPark/BP/BP_PaperCharacter.BP_PaperCharacter_C"))
  (if (not (Variables|/Game/GirafficPark/BP/BP_PaperCharacter.BP_PaperCharacter_C|GetSafePeriod _returnvalue_2))
    (if (Collision|IsOverlappingActor OverlappedComponent _returnvalue :!class /Script/Engine.PrimitiveComponent)
      (Input|DisableInput _returnvalue (Game|GetPlayerController 0))
      (Variables|/Game/GirafficPark/BP/BP_PaperCharacter.BP_PaperCharacter_C|SetLives _returnvalue_2 (- (Variables|/Game/GirafficPark/BP/BP_PaperCharacter.BP_PaperCharacter_C|GetLives _returnvalue_2) 1))
      (bind _foundwidgets (Widget|GetAllWidgetsOfClass "/Game/GirafficPark/BP/Widgets/MainGamePlayUI.MainGamePlayUI_C" true))
      (Default|UpdateText (Utilities|Array|Get(acopy) _foundwidgets))
      (Variables|/Game/GirafficPark/BP/BP_PaperCharacter.BP_PaperCharacter_C|SetSafePeriod _returnvalue_2 true)
      (Character|LaunchCharacter _returnvalue_2 (Math|Vector|MakeVector (* (.x (Math|Vector|Normalize (- (Transformation|GetActorLocation _returnvalue) (Transformation|GetActorLocation)))) (Variables|Default|GetKnockbackHorizontal)) 0.0 (Variables|Default|GetKnockbackVertical)) false false)
      (Utilities|FlowControl|Delay 0.4)
      (Input|EnableInput _returnvalue (Game|GetPlayerController 0))
      (Utilities|FlowControl|Delay 1.5)
      (Variables|/Game/GirafficPark/BP/BP_PaperCharacter.BP_PaperCharacter_C|SetSafePeriod _returnvalue_2 false))))

(event EventBeginPlay)

(event Collision|EventActorBeginOverlap
  (params (OtherActor :type Actor%20Object%20Reference)))

(event EventTick
  (params (DeltaSeconds :type Float%20%28single-precision%29))
  (if (Variables|Default|GetOverlapped)
    (Transformation|AddActorWorldOffset (* DeltaSeconds (* (Variables|Default|GetMoveDirection) (Variables|Default|GetMoveSpeed))))))

(fn ConstructionScript)