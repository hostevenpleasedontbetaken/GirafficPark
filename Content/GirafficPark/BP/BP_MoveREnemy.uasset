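; BP_MoveREnemy is an enemy actor that starts moving once the player character comes within range.
; An overlap on its ProximityCol component sets a latched Overlapped flag if the player character is touching it.
; While the flag is set, Tick offsets the actor along MoveDirection at MoveSpeed, scaled by delta time and without sweep, so movement ignores collision and never stops.
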(event OnComponentBeginOverlap(ProximityCol)
  (params (OverlappedComponent :type Primitive%20Component%20Object%20Reference) (OtherActor :type Actor%20Object%20Reference) (OtherComp :type Primitive%20Component%20Object%20Reference) (OtherBodyIndex :type Integer) (bFromSweep :type Boolean) (SweepResult :type Hit%20Result%20Structure%20%28by%20ref%29))
  (if (Collision|IsOverlappingActor OverlappedComponent (Game|GetPlayerCharacter 0) :!class /Script/Engine.PrimitiveComponent)
    (Variables|Default|SetOverlapped true)))

(event EventBeginPlay)

(event Collision|EventActorBeginOverlap
  (params (OtherActor :type Actor%20Object%20Reference)))

(event EventTick
  (params (DeltaSeconds :type Float%20%28single-precision%29))
  (if (Variables|Default|GetOverlapped)
    (Transformation|AddActorWorldOffset (* DeltaSeconds (* (Variables|Default|GetMoveDirection) (Variables|Default|GetMoveSpeed))))))

(fn ConstructionScript)