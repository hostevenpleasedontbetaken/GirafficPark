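; BP_3DGameManager sets up the game's weapon lists on BeginPlay.
; It clears AllWeapons and the game instance's unlocked lists (locked lists are not cleared), then loads every row of the Weapons data table.
; Each weapon is sorted by unlock state and type into BP_GameInstance's unlocked or locked, primary or secondary arrays.
; If the primary weapon's name is empty, the row named "Stick" becomes the default.
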(event EventBeginPlay
  (CallFunction|WeaponGameInstance))

(fn ConstructionScript)

(fn Clear
  (bind _asbp_game_instance (Utilities|Casting|CastToBP_GameInstance (Game|GetGameInstance)))
  (Utilities|Array|Clear (Variables|Default|GetAllWeapons))
  (Utilities|Array|Clear (Variables|/Game/GirafficPark/BP/BP_GameInstance.BP_GameInstance_C|GetUnlocked%20Primary _asbp_game_instance))
  (Utilities|Array|Clear (Variables|/Game/GirafficPark/BP/BP_GameInstance.BP_GameInstance_C|GetUnlocked%20Secondary _asbp_game_instance)))

(fn WeaponGameInstance
  (CallFunction|Clear)
  (bind _outrownames (DataTable|GetDataTableRowNames "/Game/GirafficPark/Data/DT/Weapons.Weapons"))
  (for _array_element _outrownames
    (bind _returnvalue (Utilities|GetDataTableRow "/Game/GirafficPark/Data/DT/Weapons.Weapons" _array_element)
      (:then
        (Utilities|Array|Add (Variables|Default|GetAllWeapons) _returnvalue)
        (if (Utilities|Enum|Equal(Enum) (.WeaponName (Utilities|Struct|BreakS_WeaponData _returnvalue)) "Stick")
          (Variables|Default|SetStick _returnvalue)))))
  (for _array_element_2 (Variables|Default|GetAllWeapons)
    (if (.Unlocked (Utilities|Struct|BreakS_WeaponData _array_element_2))
      (if (Utilities|Enum|Equal(Enum) (.Type (Utilities|Struct|BreakS_WeaponData _array_element_2)) "NewEnumerator0")
        (bind _asbp_game_instance (Utilities|Casting|CastToBP_GameInstance (Game|GetGameInstance)))
        (Utilities|Array|Add (Variables|/Game/GirafficPark/BP/BP_GameInstance.BP_GameInstance_C|GetUnlocked%20Primary _asbp_game_instance) _array_element_2)
        (else
          (bind _asbp_game_instance_2 (Utilities|Casting|CastToBP_GameInstance (Game|GetGameInstance)))
          (Utilities|Array|Add (Variables|/Game/GirafficPark/BP/BP_GameInstance.BP_GameInstance_C|GetUnlocked%20Secondary _asbp_game_instance_2) _array_element_2)))
      (elif (Utilities|Enum|Equal(Enum) (.Type (Utilities|Struct|BreakS_WeaponData _array_element_2)) "NewEnumerator0")
        (bind _asbp_game_instance_3 (Utilities|Casting|CastToBP_GameInstance (Game|GetGameInstance)))
        (Utilities|Array|Add (Variables|/Game/GirafficPark/BP/BP_GameInstance.BP_GameInstance_C|GetLocked%20Primary _asbp_game_instance_3) _array_element_2)
        (else
          (bind _asbp_game_instance_4 (Utilities|Casting|CastToBP_GameInstance (Game|GetGameInstance)))
          (Utilities|Array|Add (Variables|/Game/GirafficPark/BP/BP_GameInstance.BP_GameInstance_C|GetLocked%20Secondary _asbp_game_instance_4) _array_element_2)))))
  (bind _asbp_game_instance_5 (Utilities|Casting|CastToBP_GameInstance (Game|GetGameInstance)))
  (if (Utilities|Enum|Equal(Enum) (.WeaponName (Utilities|Struct|BreakS_WeaponData (Variables|/Game/GirafficPark/BP/BP_GameInstance.BP_GameInstance_C|GetPrimary%20Weapon _asbp_game_instance_5))) "")
    (Variables|/Game/GirafficPark/BP/BP_GameInstance.BP_GameInstance_C|SetPrimary%20Weapon _asbp_game_instance_5 (Variables|Default|GetStick))))