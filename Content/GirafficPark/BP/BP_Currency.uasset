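; BP_Currency is a money pickup that the player collects by touching it.
; When its Sphere begins an overlap and is overlapping player character 0, the actor destroys itself, then adds one to Money on BP_PaperCharacter.
; It finds that character with GetActorOfClass and calls UpdateText on the first top-level MainGamePlayUI widget, looking both up on each pickup instead of caching references.
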(event OnComponentBeginOverlap(Sphere)
  (params (OverlappedComponent :type Primitive%20Component%20Object%20Reference) (OtherActor :type Actor%20Object%20Reference) (OtherComp :type Primitive%20Component%20Object%20Reference) (OtherBodyIndex :type Integer) (bFromSweep :type Boolean) (SweepResult :type Hit%20Result%20Structure%20%28by%20ref%29))
  (if (Collision|IsOverlappingActor OverlappedComponent (Game|GetPlayerCharacter 0) :!class /Script/Engine.PrimitiveComponent)
    (Actor|DestroyActor)
    (bind _returnvalue (Actor|GetActorOfClass "/Game/GirafficPark/BP/BP_PaperCharacter.BP_PaperCharacter_C"))
    (Variables|/Game/GirafficPark/BP/BP_PaperCharacter.BP_PaperCharacter_C|SetMoney _returnvalue (+ (Variables|/Game/GirafficPark/BP/BP_PaperCharacter.BP_PaperCharacter_C|GetMoney _returnvalue) 1))
    (bind _foundwidgets (Widget|GetAllWidgetsOfClass "/Game/GirafficPark/BP/Widgets/2DLevelWidgets/MainGamePlayUI.MainGamePlayUI_C" true))
    (Default|UpdateText (Utilities|Array|Get(acopy) _foundwidgets))))

(event EventBeginPlay)

(event Collision|EventActorBeginOverlap
  (params (OtherActor :type Actor%20Object%20Reference)))

(event EventTick
  (params (DeltaSeconds :type Float%20%28single-precision%29)))

(fn ConstructionScript)