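; BP_Door is a door actor that slides slightly downward once when MoveDoor is triggered.
; On BeginPlay it searches all Button actors for the one whose DoorToConnect references this door, then stores that button and its starting location.
; MoveDoor plays a Timeline that lerps the door's location downward, unless the linked button is already pressed, and marks that button Pressed during playback.
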(event Custom|MoveDoor
  (bind _button_connected (Variables|Default|GetButton%20Connected))
  (bind _starting (Variables|Default|GetStarting))
  (bind (_x _y _z) (Math|Vector|BreakVector _starting))
  (if (not (Variables|/Game/GirafficPark/BP/Doors/Button.Button_C|GetPressed _button_connected))
    (bind _doormove (Timeline|Timeline PlayFromStart)
      (:Update
        (Transformation|SetActorLocation (Math|Vector|Lerp(Vector) (Variables|Default|GetStarting) (Math|Vector|MakeVector _x _y (- _z 1e+01)) _doormove) false false)
        (Variables|/Game/GirafficPark/BP/Doors/Button.Button_C|SetPressed _button_connected true)))))

(event EventBeginPlay
  (bind _outactors (Actor|GetAllActorsOfClass "/Game/GirafficPark/BP/Doors/Button.Button_C"))
  (for _array_element _outactors
    (if (== self (Variables|/Game/GirafficPark/BP/Doors/Button.Button_C|GetDoor%20to%20Connect _array_element))
      (Variables|Default|SetButton%20Connected _array_element)
      (Variables|Default|SetStarting (Transformation|GetActorLocation)))))

(event Collision|EventActorBeginOverlap
  (params (OtherActor :type Actor%20Object%20Reference)))

(event EventTick
  (params (DeltaSeconds :type Float%20%28single-precision%29)))

(fn ConstructionScript)