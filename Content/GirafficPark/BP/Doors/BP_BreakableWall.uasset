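; BP_BreakableWall is a wall that a dashing player character breaks through.
; On BeginPlay it holds its flipbook stopped on the first frame.
; When a BP_PaperCharacter overlaps the Box while its Dash flag is set, the flipbook plays and the actor destroys itself after the flipbook's length.
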(event OnComponentBeginOverlap(Box)
  (params (OverlappedComponent :type Primitive%20Component%20Object%20Reference) (OtherActor :type Actor%20Object%20Reference) (OtherComp :type Primitive%20Component%20Object%20Reference) (OtherBodyIndex :type Integer) (bFromSweep :type Boolean) (SweepResult :type Hit%20Result%20Structure%20%28by%20ref%29))
  (bind _paperflipbook (Variables|Default|GetPaperFlipbook))
  (bind _asbp_paper_character (Utilities|Casting|CastToBP_PaperCharacter OtherActor))
  (if (Variables|/Game/GirafficPark/BP/Player/BP_PaperCharacter.BP_PaperCharacter_C|GetDash _asbp_paper_character)
    (Audio|Components|Audio|Play _paperflipbook)
    (Utilities|FlowControl|Delay (Class|PaperFlipbookComponent|GetFlipbookLength _paperflipbook))
    (Actor|DestroyActor)))

(event EventBeginPlay
  (bind _paperflipbook (Variables|Default|GetPaperFlipbook))
  (Class|PaperFlipbookComponent|SetPlaybackPositioninFrames _paperflipbook 0 false)
  (Audio|Components|Audio|Stop _paperflipbook))

(event Collision|EventActorBeginOverlap
  (params (OtherActor :type Actor%20Object%20Reference)))

(event EventTick
  (params (DeltaSeconds :type Float%20%28single-precision%29)))

(fn ConstructionScript)