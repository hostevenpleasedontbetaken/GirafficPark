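; BP_Player is the player's marker on the level select map, travelling between map points and opening the pause menu.
; On BeginPlay it restores a position from BP_GameInstance: the last move's start if the level was lost, otherwise its end.
; MoveToPoint lerps it along a timeline at a height offset, saving both positions to the game instance.
; On arrival, it passes the matching BP_MapPoints level info to W_MainLevelSelect.
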(event Custom|MoveToPoint
  (params (PointLocation :type Vector) (Level%20Name :type String))
  (Variables|Default|SetEndPoint PointLocation)
  (Variables|Default|SetStartPoint (Transformation|GetActorLocation))
  (bind _newtrack_0 (Timeline|MovementTimeline PlayFromStart)
    (:Update
      (Transformation|SetActorLocation (Math|Vector|Lerp(Vector) (Math|Vector|MakeVector (.x (Variables|Default|GetStartPoint)) (.y (Variables|Default|GetStartPoint)) (+ (.z (Variables|Default|GetStartPoint)) 45.0)) (Math|Vector|MakeVector (.x (Variables|Default|GetEndPoint)) (.y (Variables|Default|GetEndPoint)) (+ (.z (Variables|Default|GetEndPoint)) 45.0)) _newtrack_0) false false)
      (bind _asbp_game_instance (Utilities|Casting|CastToBP_GameInstance (Game|GetGameInstance)))
      (Variables|/Game/GirafficPark/BP/BP_GameInstance.BP_GameInstance_C|SetPlayerEndPos _asbp_game_instance (Math|Vector|Lerp(Vector) (Math|Vector|MakeVector (.x (Variables|Default|GetStartPoint)) (.y (Variables|Default|GetStartPoint)) (+ (.z (Variables|Default|GetStartPoint)) 45.0)) (Math|Vector|MakeVector (.x (Variables|Default|GetEndPoint)) (.y (Variables|Default|GetEndPoint)) (+ (.z (Variables|Default|GetEndPoint)) 45.0)) _newtrack_0))
      (Variables|/Game/GirafficPark/BP/BP_GameInstance.BP_GameInstance_C|SetPlayerStartPos _asbp_game_instance (Variables|Default|GetStartPoint)))
    (:Finished
      (bind _outactors (Actor|GetAllActorsOfClass "/Game/GirafficPark/BP/LevelBPS/BP_MapPoints.BP_MapPoints_C"))
      (for _array_element _outactors
        (if (Utilities|Enum|Equal(Enum) Level%20Name (.LevelName (Utilities|Struct|BreakLevelInfo (Variables|/Game/GirafficPark/BP/LevelBPS/BP_MapPoints.BP_MapPoints_C|GetLevelInfo _array_element))))
          (bind _foundwidgets (Widget|GetAllWidgetsOfClass "/Game/GirafficPark/BP/Widgets/LevelSelectWidgets/W_MainLevelSelect.W_MainLevelSelect_C" true))
          (Default|UpdateInformation (Utilities|Array|Get(acopy) _foundwidgets) (.LevelBeat (Utilities|Struct|BreakLevelInfo (Variables|/Game/GirafficPark/BP/LevelBPS/BP_MapPoints.BP_MapPoints_C|GetLevelInfo _array_element))) (.LevelName (Utilities|Struct|BreakLevelInfo (Variables|/Game/GirafficPark/BP/LevelBPS/BP_MapPoints.BP_MapPoints_C|GetLevelInfo _array_element)))))))))

(event EventBeginPlay
  (bind _asbp_game_instance (Utilities|Casting|CastToBP_GameInstance (Game|GetGameInstance)))
  (if (Variables|/Game/GirafficPark/BP/BP_GameInstance.BP_GameInstance_C|GetLevelLost _asbp_game_instance)
    (Transformation|SetActorLocation (Variables|/Game/GirafficPark/BP/BP_GameInstance.BP_GameInstance_C|GetPlayerStartPos _asbp_game_instance) false false)
    (else
      (Transformation|SetActorLocation (Variables|/Game/GirafficPark/BP/BP_GameInstance.BP_GameInstance_C|GetPlayerEndPos _asbp_game_instance) false false))))

(event Input|ActionEvents|InputActionOpenMenu
  (params (Key :type Key%20Structure :default "None"))
  (:Pressed
    (Viewport|RemoveAllWidgets)
    (Game|SetGamePaused true)
    (bind _returnvalue (UserInterface|CreateWidget "/Game/GirafficPark/BP/Widgets/LevelSelectPause.LevelSelectPause_C"))
    (UserInterface|Viewport|AddtoViewport _returnvalue 0)))

(fn ConstructionScript)