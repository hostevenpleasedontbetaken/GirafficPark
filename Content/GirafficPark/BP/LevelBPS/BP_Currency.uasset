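; BP_Currency is a food pellet pickup that the player collects by touching it.
; When its sphere overlaps the player character, it destroys itself, then increments FoodPellets and FPPConversion on BP_GameInstance.
; It then refreshes the first MainGamePlayUI widget found through UpdateText and calls UpdateElongated on the player's BP_PaperCharacter.
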(event OnComponentBeginOverlap(Sphere)
  (params (OverlappedComponent :type Primitive%20Component%20Object%20Reference) (OtherActor :type Actor%20Object%20Reference) (OtherComp :type Primitive%20Component%20Object%20Reference) (OtherBodyIndex :type Integer) (bFromSweep :type Boolean) (SweepResult :type Hit%20Result%20Structure%20%28by%20ref%29))
  (bind _returnvalue (Game|GetPlayerCharacter 0))
  (if (Collision|IsOverlappingActor OverlappedComponent _returnvalue :!class /Script/Engine.PrimitiveComponent)
    (Actor|DestroyActor)
    (bind _asbp_game_instance (Utilities|Casting|CastToBP_GameInstance (Game|GetGameInstance)))
    (Variables|/Game/GirafficPark/BP/BP_GameInstance.BP_GameInstance_C|SetFood%20Pellets _asbp_game_instance (+ (Variables|/Game/GirafficPark/BP/BP_GameInstance.BP_GameInstance_C|GetFood%20Pellets _asbp_game_instance) 1))
    (Variables|/Game/GirafficPark/BP/BP_GameInstance.BP_GameInstance_C|SetFPPConversion _asbp_game_instance (+ (Variables|/Game/GirafficPark/BP/BP_GameInstance.BP_GameInstance_C|GetFPPConversion _asbp_game_instance) 1))
    (bind _foundwidgets (Widget|GetAllWidgetsOfClass "/Game/GirafficPark/BP/Widgets/2DLevelWidgets/MainGamePlayUI.MainGamePlayUI_C" true))
    (Default|UpdateText (Utilities|Array|Get(acopy) _foundwidgets))
    (bind _asbp_paper_character (Utilities|Casting|CastToBP_PaperCharacter _returnvalue))
    (Default|UpdateElongated _asbp_paper_character)))

(event EventBeginPlay)

(event Collision|EventActorBeginOverlap
  (params (OtherActor :type Actor%20Object%20Reference)))

(event EventTick
  (params (DeltaSeconds :type Float%20%28single-precision%29)))

(fn ConstructionScript)